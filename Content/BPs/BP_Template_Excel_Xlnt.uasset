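; Template Blueprint that tests reading Excel .xlsx workbooks through an XLNT plugin.
; On BeginPlay it opens a hard-coded local workbook, requests all worksheets through a delegate event, and prints each sheet title on success.
; A disconnected alternative using LoadExcel and AllSheets, plus unused worksheet title, ID and index getters in a Samples graph, remain for reference.
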(event Custom|Delegate_Worksheets
  (params (IsSuccessfull :type Boolean) (Out_Sheets :type Array%20of%20Xlnt%20Worksheet%20Structures))
  (if IsSuccessfull
    (for _array_element Out_Sheets
      (Development|PrintString (.title _array_element) true true "(R=0.000000,G=0.660000,B=1.000000,A=1.000000)" 3e+01))))

(event EventBeginPlay
  (bind (_out_doc _returnvalue) (Class|FFExcelBPLibrary|XLNTOpenExcelFile "C:\\Users\\erayo\\Downloads\\Maxion\\Haziran_2023_duruş.xlsx"))
  (if _returnvalue
    (Class|FFExcelBPLibrary|XLNTWorksheetsGetAll (delegate Custom|Delegate_Worksheets) _out_doc)))

(fn ConstructionScript)